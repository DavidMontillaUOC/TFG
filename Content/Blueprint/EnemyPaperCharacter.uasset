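; Paper2D enemy character that fires magic projectiles at the player while its detection Sphere is overlapped.
; Sphere begin and end overlaps toggle SeesPlayer without checking which actor overlapped.
; Tick calls ShotPlayer, which spawns BP_Ranged_Weapon_Magic at the enemy's location, aimed at player character 0.
; An IsShooting flag, cleared by a short Delay in the else branch, throttles the fire rate.
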(event OnComponentBeginOverlap(Sphere)
  (params (OverlappedComponent :type Primitive%20Component%20Object%20Reference) (OtherActor :type Actor%20Object%20Reference) (OtherComp :type Primitive%20Component%20Object%20Reference) (OtherBodyIndex :type Integer) (bFromSweep :type Boolean) (SweepResult :type Hit%20Result%20Structure%20%28by%20ref%29))
  (Variables|Default|SetseesPlayer true))

(event OnComponentEndOverlap(Sphere)
  (params (OverlappedComponent :type Primitive%20Component%20Object%20Reference) (OtherActor :type Actor%20Object%20Reference) (OtherComp :type Primitive%20Component%20Object%20Reference) (OtherBodyIndex :type Integer))
  (Variables|Default|SetseesPlayer false))

(event Custom|ShotPlayer
  (if (and (Variables|Default|GetseesPlayer) (not (Variables|Default|GetisShooting)))
    (Variables|Default|SetisShooting true)
    (Game|SpawnActorfromClass "/Game/Character/Weapons/RangedWeapons/BP_Ranged_Weapon_Magic.BP_Ranged_Weapon_Magic_C" (Math|Transform|MakeTransform (.location (Transformation|GetActorTransform self)) (Math|Conversions|RotationFromXVector (- (Transformation|GetActorLocation (Game|GetPlayerCharacter 0)) (Transformation|GetActorLocation self))) "1.000000,1.000000,1.000000") "AlwaysSpawn" "MultiplyWithRoot" 0 0)
    (else
      (Utilities|FlowControl|Delay 0.5)
      (Variables|Default|SetisShooting false))))

(event EventBeginPlay
  (Variables|Default|SetseesPlayer false))

(event Collision|EventActorBeginOverlap
  (params (OtherActor :type Actor%20Object%20Reference)))

(event EventTick
  (params (DeltaSeconds :type Float%20%28single-precision%29))
  (CallFunction|ShotPlayer))

(fn ConstructionScript)